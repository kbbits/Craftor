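; World grid manager that stores placed blocks as instanced meshes and snaps world locations to the block grid.
; AddPlaceableBlock finds the hierarchical instanced mesh component for the placeable's class, or creates one with its body mesh, then adds an instance at the given transform.
; GridifyWorldLocation rounds each axis to the base block size, leaving the block extent input unused.
; RemoveAll clears the instances on every block component.
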(fn ConstructionScript)

(fn AddPlaceableBlock
  (params (Placeable :type Placeable%20Block%20Base%20Object%20Reference) (Transform :type Transform))
  (bind _returnvalue (Utilities|GetClass Placeable))
  (Utilities|FlowControl|Sequence
    (:then_0
      (bind (_found _block_hismc) (CallFunction|HISMCforBlockType _returnvalue))
      (if _found
        (LocalVariables|SetBlock%20HISMC _block_hismc)
        (else
          (bind _returnvalue_2 (AddComponent|AddBlockHISMC :PlaceableBlockClass _returnvalue))
          (bind _output_get (LocalVariables|SetBlock%20HISMC _returnvalue_2))
          (Components|StaticMesh|SetStaticMesh _output_get (Variables|/Script/Engine.StaticMeshComponent|GetStaticMesh (Variables|/Game/Craftor/Placeables/Placeable_Base.Placeable_Base_C|GetBodyMesh Placeable))))))
    (:then_1
      (Class|InstancedStaticMeshComponent|AddInstanceWorldSpace (LocalVariables|GetBlock%20HISMC) Transform))))

(fn HISMCforBlockType
  (params (InputPin :type Placeable%20Block%20Base%20Class%20Reference))
  (bind _array_element (Utilities|Array|ForEachLoopwithBreak (Actor|GetComponentsByClass "/Game/Craftor/Placeables/Blocks/Block_HISMC.Block_HISMC_C") :!label _label)
    (:LoopBody
      (if (== (Variables|/Game/Craftor/Placeables/Blocks/Block_HISMC.Block_HISMC_C|GetPlaceableBlockClass _array_element) InputPin)
        (LocalVariables|SetTmp%20HISMC _array_element)
        (goto _label Break)))
    (:Completed
      (return (Utilities|IsValid (LocalVariables|GetTmp%20HISMC)) (LocalVariables|GetTmp%20HISMC)))))

(fn GridifyWorldLocation
  (params (Location :type Vector) (Block%20Extent :type Vector))
  (bind (_x _y _z) (Math|Vector|BreakVector Location))
  (bind _block_base_size (Variables|Default|GetBlock%20Base%20Size))
  (return (Math|Vector|MakeVector (Math|Float|SnapToGrid(Float) _x _block_base_size) (Math|Float|SnapToGrid(Float) _y _block_base_size) (Math|Float|SnapToGrid(Float) _z _block_base_size))))

(fn RemoveAll
  (for _array_element (Actor|GetComponentsByClass "/Game/Craftor/Placeables/Blocks/Block_HISMC.Block_HISMC_C")
    (Components|InstancedStaticMesh|ClearInstances _array_element)))