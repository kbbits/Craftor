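; Base actor for Craftor placeables, handling ghost preview, placement validation and unplacing through IPlaceable.
; On spawn or unplace it hides "PlaceableBody"-tagged meshes behind runtime ghost copies; placing restores visibility and collision.
; Hit results are validated by placeability mode (any surface, horizontal, surface type or world grid), switching the ghost's glow material.
; The returned location is offset along the hit normal by body bounds, snapped via WorldGridManager in grid mode.
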(event EventOnPlaceableSpawn
  ;[1 1 1] On Placeable Spawn (IPlaceable) - when actor spawns in world
  (CallFunction|ShowGhost))

(event EventOnPlaced
  ;[1 1 1] On Placed (IPlaceable) - when placeable is placed
  (CallFunction|HideGhost)
  (Variables|Default|SetPlaced? true))

(fn ConstructionScript)

(fn GetCraftorPlayerController
  (bind _ascraftor_player_controller (Utilities|Casting|CastToCraftorPlayerController (Game|GetPlayerController 0)))
  (return _ascraftor_player_controller (Utilities|IsValid _ascraftor_player_controller)))

(fn ShowGhost
  (for _array_element (Actor|GetComponentsbyTag "/Script/Engine.StaticMeshComponent" "PlaceableBody")
    (Utilities|IsValid _array_element
      (:Is%20Valid
        (Rendering|SetVisibility _array_element false true)
        (Collision|SetCollisionEnabled _array_element "NoCollision")
        (bind _returnvalue (AddComponent|AddStaticMeshComponent true (Transformation|GetRelativeTransform _array_element)))
        (Transformation|AttachComponentToComponent _returnvalue (Transformation|GetAttachParent (Variables|Default|GetBodyMesh)) "None" "KeepRelative" "KeepRelative" "KeepRelative" false)
        (Components|StaticMesh|SetStaticMesh _returnvalue (Variables|/Script/Engine.StaticMeshComponent|GetStaticMesh _array_element))
        (Rendering|Material|SetMaterial _returnvalue 0 "/Game/Craftor/Assets/Materials/M_Ghost_Glow_Red.M_Ghost_Glow_Red")
        (Rendering|SetVisibility _returnvalue true true)
        (Physics|SetSimulatePhysics _returnvalue false)
        (Collision|SetCollisionEnabled _returnvalue "NoCollision")
        (Utilities|Array|Add (Variables|Default|GetGhostMeshes) _returnvalue))))
  (return))

(fn HideGhost
  (Utilities|FlowControl|Sequence
    (:then_0
      ;[1 1 1] Remove Ghosts
      (for _array_element (Variables|Default|GetGhostMeshes)
        (Rendering|SetVisibility _array_element false true)
        (Components|DestroyComponent _array_element))
      (Utilities|Array|Clear (Variables|Default|GetGhostMeshes)))
    (:then_1
      ;[1 1 1] Reset PlaceableBody Meshes
      (for _array_element_2 (Actor|GetComponentsbyTag "/Script/Engine.StaticMeshComponent" "PlaceableBody")
        (Rendering|SetVisibility _array_element_2 true true)
        (Collision|SetCollisionEnabled _array_element_2 "QueryAndPhysics")))
    (:then_2
      (return))))

(fn UpdateGhost
  (params (CurrentlyPlaceable? :type Boolean))
  (if (Math|Boolean|NotEqual(Boolean) CurrentlyPlaceable? (Variables|Default|GetPlaceableAtLocation?))
    (for _array_element (Variables|Default|GetGhostMeshes)
      (Rendering|Material|SetMaterial _array_element 0 (select CurrentlyPlaceable? "/Game/Craftor/Assets/Materials/M_Ghost_Glow.M_Ghost_Glow" "/Game/Craftor/Assets/Materials/M_Ghost_Glow_Red.M_Ghost_Glow_Red")))
    (Variables|Default|SetPlaceableAtLocation? CurrentlyPlaceable?)))

(fn AllowDeconstruct
  (return (Variables|Default|GetAllow%20Deconstruct?)))

(fn GetPlaceability
  (bind _surface_type (CallFunction|GetPlaceableSurfaceType))
  (return (Variables|Default|GetPlaceability) _surface_type))

(fn GetPlaceableSurfaceType
  (return (Variables|Default|GetPlaceabilitySurfaceType)))

(fn GetRequiredInventory
  (return (Variables|Default|GetRequiredBuildable)))

(fn GetThumbnail
  (return (Utilities|Struct|BreakTextureInfo (Variables|Default|GetThumbnail%20Info))))

(fn IsPlaceablebyHit?
  (params (Hit :type Hit%20Result%20Structure) (World%20Grid%20Manager :type World%20Grid%20Manager%20BP%20Object%20Reference))
  (bind (_bblockinghit _binitialoverlap _time _distance _location _impactpoint _normal _impactnormal _physmat _hitactor) (Collision|BreakHitResult Hit))
  (Utilities|FlowControl|Sequence
    (:then_0
      (switch Utilities|FlowControl|Switch|SwitchonPlaceability (Variables|Default|GetPlaceability)
        (:NewEnumerator1
          (Utilities|IsValid _hitactor
            (:Is%20Not%20Valid
              (LocalVariables|SetTmpPlaceable? false :!label _label))))
        (:NewEnumerator2
          (if (not (Math|Vector|Equal(Vector) (Math|Vector|Normalize _impactnormal) "0, 0,1.000000" 0.001))
            (goto _label)))
        (:NewEnumerator3
          (if (Utilities|DoesObjectImplementInterface _hitactor "/Game/Craftor/PlaceableSurfaces/IPlaceableSurface.IPlaceableSurface_C")
            (bind _allowed (Class|IPlaceableSurface|AllowsSurfaceType?(Message) _hitactor (Variables|Default|GetPlaceabilitySurfaceType)))
            (if (not _allowed)
              (goto _label))
            (else
              (goto _label))))
        (:NewEnumerator4
          (Utilities|IsValid World%20Grid%20Manager
            (:Is%20Not%20Valid
              (LocalVariables|SetTmpPlaceable? false))))))
    (:then_1
      ;[1 1 1] Return
      (return (LocalVariables|GetTmpPlaceable?)))))

(fn IsPlaced?
  (return (Variables|Default|GetPlaced?)))

(fn OnUnplaced
  (Utilities|FlowControl|Sequence
    (:then_0
      (if (Variables|Default|GetPlaced?)
        (CallFunction|ShowGhost)
        (Variables|Default|SetPlaced? false)
        (LocalVariables|Setdid_unplace? true)))
    (:then_1
      (return (LocalVariables|Getdid_unplace?) true))))

(fn PlaceableLocationbyHit
  (params (Hit :type Hit%20Result%20Structure) (World%20Grid%20Manager :type World%20Grid%20Manager%20BP%20Object%20Reference))
  (bind (_bblockinghit _binitialoverlap _time _distance _location _impactpoint _normal _impactnormal _physmat _hitactor _hitcomponent _hitbonename _hititem _faceindex _tracestart _traceend) (Collision|BreakHitResult Hit))
  (bind _bodymesh (Variables|Default|GetBodyMesh))
  (bind _boxextent (Collision|GetComponentBounds _bodymesh))
  (bind _returnvalue (* _normal _boxextent))
  (bind _returnvalue_2 (+ _location _returnvalue))
  (bind _returnvalue_3 (Math|Vector|SelectVector _returnvalue_2 _traceend _bblockinghit))
  (bind _is_placeable_ (CallFunction|IsPlaceablebyHit? Hit World%20Grid%20Manager))
  (if (Utilities|Enum|Equal(Enum) (Variables|Default|GetPlaceability) "NewEnumerator4")
    (CallFunction|UpdateGhost _is_placeable_)
    (return _is_placeable_ (Default|GridifyWorldLocation World%20Grid%20Manager _returnvalue_3 _boxextent))
    (else
      (CallFunction|UpdateGhost _is_placeable_)
      (return _is_placeable_ _returnvalue_3))))